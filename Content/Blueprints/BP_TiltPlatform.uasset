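; BP_TiltPlatform is a player-tilted platform viewed through a static camera.
; On BeginPlay it finds the BP_StaticCamera actor and makes it the first player controller's view target.
; IA_Tilt input, scaled by TiltSpeed, sets a target roll and pitch, which resets to level on release.
; Tick eases the rotation toward that target with RInterpTo at ReturnSpeed, for both tilting and returning.
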(event Input|EnhancedActionEvents|EnhancedInputActionIA_Tilt
  (params (ActionValue :type Vector%202D%20Structure) (ElapsedSeconds :type Float%20%28double-precision%29) (TriggeredSeconds :type Float%20%28double-precision%29) (InputAction :type Input%20Action%20Object%20Reference :default "/Game/Input/TiltingMaze/IA_Tilt.IA_Tilt"))
  (:Triggered
    (Variables|Default|SetTargetRotation (Math|Rotator|MakeRotator (* (Variables|Default|GetTiltSpeed) (.x ActionValue)) (* (.y ActionValue) (Variables|Default|GetTiltSpeed)) 0.0)))
  (:Completed
    (Variables|Default|SetTargetRotation "0, 0, 0")))

(event EventTick
  (params (DeltaSeconds :type Float%20%28single-precision%29))
  (bind _output_get (Variables|Default|SetCurrentRotation (Math|Interpolation|RInterpTo (Variables|Default|GetCurrentRotation) (Variables|Default|GetTargetRotation) DeltaSeconds (Variables|Default|GetReturnSpeed))))
  (Transformation|SetActorRotation _output_get))

(event EventBeginPlay
  (bind _returnvalue (Actor|GetActorOfClass "/Game/Blueprints/BP_StaticCamera.BP_StaticCamera_C"))
  (bind _output_get (Variables|Default|SetCamera _returnvalue))
  (Game|Player|SetViewTargetwithBlend (Game|GetPlayerController 0) _output_get 0.0 "VTBlend_Linear" 0.0 false))

(fn ConstructionScript)